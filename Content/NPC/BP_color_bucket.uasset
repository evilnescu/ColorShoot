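; BP_color_bucket is an NPC that carries a random color, chases the player and shows its life as size.
; When it overlaps a weaker bucket, it takes a point of life and blends slightly toward that color.
; Overlapping the player runs a timeline that blends the player's color toward its own, costing the bucket life on completion.
; Tick updates material and scale and destroys it at low life.
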(event `self.ReceiveBeginPlay`
  (set `self.COLOR` (`KismetMathLibrary.Conv_VectorToLinearColor` (`KismetMathLibrary.RandomUnitVector`)))
  (`MeshComponent.SetVectorParameterValueOnMaterials` (`self.Sphere`) "DIFF-color" (`KismetMathLibrary.Conv_LinearColorToVector` (`self.COLOR`)))
  (if (`self.Is_NPC_Alive`) :!label _label
    (`|AIMoveTo` self (0.0 0.0 0.0) (`GameplayStatics.GetPlayerCharacter` 0) 1.0
      (:`OnSuccess`
        _)
      (:`OnFail`
        _))
    (`KismetSystemLibrary.Delay` 0.2)
    (goto _label)))

(event `self.ReceiveTick`
  (params (DeltaSeconds :type "Float (single-precision)"))
  (bind _returnvalue (/ (`self.LIFE`) 100.0))
  ;[1 1 1] set material according to color
  (`MeshComponent.SetVectorParameterValueOnMaterials` (`self.Sphere`) "DIFF-color" (`KismetMathLibrary.Conv_LinearColorToVector` (`self.COLOR`)))
  ;[1 1 1] set scale according to life
  (`SceneComponent.SetWorldScale3D` (`self.Sphere`) (`KismetMathLibrary.MakeVector` _returnvalue _returnvalue _returnvalue))
  (`SceneComponent.SetWorldScale3D` (`self.CapsuleComponent`) (`KismetMathLibrary.MakeVector` _returnvalue _returnvalue _returnvalue))
  (`SceneComponent.SetWorldScale3D` (`self.Sphere collision`) (`KismetMathLibrary.MakeVector` _returnvalue _returnvalue _returnvalue))
  ;[1 1 1] dead
  (if (< (`self.LIFE`) 20.0)
    (set `self.DEAD` false)
    (`self.K2_DestroyActor`)))

(event `self.OnLaunched`
  (params (LaunchVelocity :type "Vector Structure") (bXYOverride :type Boolean) (bZOverride :type Boolean))
  (`MovementComponent.StopMovementImmediately` (`self.CharacterMovement`)))

(event `self.ReceiveAnyDamage`
  (params (Damage :type "Float (single-precision)") (DamageType :type "DamageType Object Reference") (InstigatedBy :type "Controller Object Reference") (DamageCauser :type "Actor Object Reference"))
  (set `self.LIFE` (- (`self.LIFE`) Damage)))

(event `self.ReceiveActorBeginOverlap`
  (params (OtherActor :type "Actor Object Reference"))
  (bind _asbp_color_bucket (cast `/Game/NPC/BP_color_bucket` OtherActor)
    (:`then`
      (if (> (`self.LIFE`) (`/Game/NPC/BP_color_bucket.LIFE` _asbp_color_bucket))
        (`KismetSystemLibrary.DrawDebugLine` (`self.K2_GetActorLocation`) (`self.K2_GetActorLocation` _asbp_color_bucket) (`self.COLOR`) 3.0 4.0)
        (set `self.COLOR` (`KismetMathLibrary.LinearColorLerp` (`self.COLOR`) (`/Game/NPC/BP_color_bucket.COLOR` _asbp_color_bucket) 0.1))
        (`/Engine/EditorBlueprintResources/StandardMacros.DecrementFloat` (`/Game/NPC/BP_color_bucket.LIFE` _asbp_color_bucket)
          (:`  `
            (`/Engine/EditorBlueprintResources/StandardMacros.IncrementFloat` (`self.LIFE`))))))
    (:`CastFailed`
      (bind _asthird_person_character (cast `/Game/ThirdPersonBP/Blueprints/ThirdPersonCharacter` OtherActor))
      (`KismetSystemLibrary.DrawDebugLine` (`self.K2_GetActorLocation`) (`self.K2_GetActorLocation` _asthird_person_character) (struct :`R` 1.0 :`G` 1.0 :`B` 1.0 :`A` 1.0) 1.0 4.0)
      (bind (_direction _lerp_amount) (`Timeline|Change Color 0 to 1 over 7sec` :!label _label_2)
        (:`Update`
          (set `/Game/ThirdPersonBP/Blueprints/ThirdPersonCharacter.COLOR` (`KismetMathLibrary.LinearColorLerp` (`/Game/ThirdPersonBP/Blueprints/ThirdPersonCharacter.COLOR` _asthird_person_character) (`self.COLOR`) _lerp_amount) _asthird_person_character))
        (:`Finished`
          (`/Engine/EditorBlueprintResources/StandardMacros.DecrementFloat` (`self.LIFE`) (* 100 _lerp_amount)))))))

(event `self.ReceiveActorEndOverlap`
  (params (OtherActor :type "Actor Object Reference"))
  (goto _label_2 :!via `Stop`))

(fn `Is_NPC_Alive`
  (returns (ReturnValue :type Boolean))
  (return (not (`self.DEAD`))))

(fn `UserConstructionScript`)