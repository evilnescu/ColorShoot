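; A color-matching goal portal that checks whether the overlapping ThirdPersonCharacter carries a color close enough to its target.
; The construction script derives the target color from a random unit vector and tints the cube's material with it.
; On overlap, the distance between the two colors decides a printed win or retry message showing that distance.
; A win also launches every BP_color_bucket actor upward.
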(event `self.ReceiveActorBeginOverlap`
  (params (OtherActor :type "Actor Object Reference"))
  (bind _asthird_person_character (cast `/Game/ThirdPersonBP/Blueprints/ThirdPersonCharacter` OtherActor))
  (bind _returnvalue (`KismetMathLibrary.LinearColor_Distance` (`self.WIN-COLOR`) (`/Game/ThirdPersonBP/Blueprints/ThirdPersonCharacter.COLOR` _asthird_person_character)))
  (if (<= _returnvalue 1.0)
    (bind _returnvalue_2 (`KismetStringLibrary.Conv_DoubleToString` _returnvalue))
    (`KismetSystemLibrary.PrintString` (`KismetStringLibrary.Concat_StrStr` "YOU WIN! " _returnvalue_2) true true (struct :`R` 0.122312 :`G` 1.0 :`A` 1.0) 5.0)
    (bind _outactors (`GameplayStatics.GetAllActorsOfClass` "/Game/NPC/BP_color_bucket.BP_color_bucket_C"))
    (for _array_element _outactors
      (`Character.LaunchCharacter` _array_element (0.0 0.0 2000.0) true true))
    (else
      (`KismetSystemLibrary.PrintString` (`KismetStringLibrary.Concat_StrStr` "TRY AGAIN...... " _returnvalue_2) true true (struct :`R` 1.0 :`A` 1.0) 5.0))))

(fn `UserConstructionScript`
  (bind _output_get (set `self.WIN-COLOR` (`KismetMathLibrary.Conv_VectorToLinearColor` (`KismetMathLibrary.RandomUnitVector`))))
  (`MeshComponent.SetVectorParameterValueOnMaterials` (`self.Cube`) "MAN-color" (`KismetMathLibrary.Conv_LinearColorToVector` _output_get)))